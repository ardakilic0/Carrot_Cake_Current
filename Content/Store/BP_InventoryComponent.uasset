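; BP_InventoryComponent is an inventory component that tracks item quantities by ItemID in InventoryMap.
; AddToInventory adds the given quantity to an existing entry's count, or creates a new entry when the ID is absent.
; It is the only active logic, with no removal, stack limit or validation; BeginPlay and Tick are disabled placeholders.
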(fn `AddToInventory`
  (params (ItemID :type Integer) (Quantity :type Integer))
  (bind (_value _returnvalue) (`BlueprintMapLibrary.Map_Find` (`self.InventoryMap`) ItemID))
  (if _returnvalue
    (`BlueprintMapLibrary.Map_Add` (`self.InventoryMap`) (`local.ItemID`) (+ Quantity _value))
    (else
      (`BlueprintMapLibrary.Map_Add` (`self.InventoryMap`) (`local.ItemID`) (`local.Quantity`))))
  (return))